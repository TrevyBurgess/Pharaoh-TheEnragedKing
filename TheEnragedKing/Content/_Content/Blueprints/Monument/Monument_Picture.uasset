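; Monument Blueprint that displays a framed picture with a 3D text name and a left and right light.
; The construction script applies the picture, frame and monument materials, sets the text from DisplayName and gives both lights a shared intensity, so each instance is configured through variables.
; At runtime, a box collision overlap only prints a debug string, and the DisplayFont variable is unused.
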(event OnComponentBeginOverlap(BoxCollision)
  (params (OverlappedComponent :type Primitive%20Component%20Object%20Reference) (OtherActor :type Actor%20Object%20Reference) (OtherComp :type Primitive%20Component%20Object%20Reference) (OtherBodyIndex :type Integer) (bFromSweep :type Boolean) (SweepResult :type Hit%20Result%20Structure%20%28by%20ref%29))
  (Development|PrintString "Collided with"))

(event EventBeginPlay)

(event Collision|EventActorBeginOverlap
  (params (OtherActor :type Actor%20Object%20Reference)))

(event EventTick
  (params (DeltaSeconds :type Float%20%28single-precision%29)))

(fn ConstructionScript
  (Rendering|Material|SetMaterial (Variables|Default|GetCanvas) 0 (Variables|Settings|GetPicture))
  (Rendering|Material|SetMaterial (Variables|Default|GetFrame) 0 (Variables|Settings|GetFrame_Mat))
  (Rendering|Material|SetMaterial (Variables|Default|GetMonument) 0 (Variables|Settings|GetMonument_Mat))
  (Variables|/Script/Text3D.Text3DComponent|SetText (Variables|Default|GetText3D) (Variables|Settings|GetDisplay_Name))
  (Rendering|Components|Light|SetIntensity (Variables|Default|GetLeft_Light) (Variables|Settings|GetIntensity))
  (Rendering|Components|Light|SetIntensity (Variables|Default|GetRight_Light) (Variables|Settings|GetIntensity)))